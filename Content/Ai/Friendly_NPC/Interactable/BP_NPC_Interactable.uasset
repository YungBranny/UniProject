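; BP_NPC_Interactable is a friendly NPC that shows a text prompt when the Astra player character is within interaction range.
; The prompt starts hidden and rotates each tick to face the player.
; Entering the box collision shows the prompt and sets Astra's CanInteract flag.
; Leaving it hides the prompt, clears the interact and speaking flags, and hides and resets Astra's dialogue window and dialogue index.
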(event `self.ReceiveBeginPlay`
  ;[1 1 1] TextRender not visible.
  (`SceneComponent.SetVisibility` (`self.TR_Interact`) false false))

(event `self.ReceiveTick`
  (params (DeltaSeconds :type "Float (single-precision)"))
  (bind _tr_interact (`self.TR_Interact`))
  ;[1 1 1] Set rotation of TR_Interact to face the player
  (`SceneComponent.K2_SetWorldRotation` _tr_interact (`KismetMathLibrary.FindLookAtRotation` (`SceneComponent.K2_GetComponentLocation` _tr_interact) (`self.K2_GetActorLocation` (`GameplayStatics.GetPlayerCharacter` 0))) false false))

(event `self.BC_Interactable.OnComponentBeginOverlap`
  (params (OverlappedComponent :type "PrimitiveComponent Object Reference") (OtherActor :type "Actor Object Reference") (OtherComp :type "PrimitiveComponent Object Reference") (OtherBodyIndex :type Integer) (bFromSweep :type Boolean) (SweepResult :type "HitResult Structure (by ref)"))
  ;[1 1 1] TR_Interact visible once the player is in the box collision.
  (bind _asastra (cast `/Game/Astra/Astra` OtherActor))
  (`SceneComponent.SetVisibility` (`self.TR_Interact`) true false)
  ;[1 1 1] Set canInteract, to see if the player can interact with the NPC.
  (set `/Game/Astra/Astra.canInteract` true _asastra))

(event `self.BC_Interactable.OnComponentEndOverlap`
  (params (OverlappedComponent :type "PrimitiveComponent Object Reference") (OtherActor :type "Actor Object Reference") (OtherComp :type "PrimitiveComponent Object Reference") (OtherBodyIndex :type Integer))
  ;[1 1 1] TR_Interact not visible once the player is out of the box collision.
  (bind _asastra (cast `/Game/Astra/Astra` OtherActor))
  (`SceneComponent.SetVisibility` (`self.TR_Interact`) false false)
  ;[1 1 1] Set canInteract, to see if the player can interact with the NPC.
  (set `/Game/Astra/Astra.canInteract` false _asastra)
  ;[1 1 1] set isSpeaking to false
  (set `/Game/Astra/Astra.isSpeaking` false _asastra)
  (bind _w_dialoguewindow (`/Game/Astra/Astra.W_DialogueWindow` _asastra))
  ;[1 1 1] Reset values in the dialogue window
  ;;[1 1 1] Set the letter count to 0, to make sure that the index is at 0 when animating the text again.
  (set `/Game/Ai/Friendly_NPC/Interactable/Interactable_Widgets/W_DialogueWindow.letterCount` 0 _w_dialoguewindow)
  ;;[1 1 1] Set the current text (what is displayed) to nothing, so new text isn't added onto what it previously was
  (set `/Game/Ai/Friendly_NPC/Interactable/Interactable_Widgets/W_DialogueWindow.currentText` "" _w_dialoguewindow)
  ;[1 1 1] Set W_DialogueWindow visibility to hidden.
  (`Widget.SetVisibility` (`/Game/Astra/Astra.W_DialogueWindow` _asastra) "Hidden")
  ;[1 1 1] Reset NPCDialogueIndex to -1, so when speaking to an Interactable NPC, dialogue resets to the first in array.
  (set `/Game/Astra/Astra.NPCDialogueIndex` -1 _asastra))

(fn `UserConstructionScript`)