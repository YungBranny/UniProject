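; NPC Blueprint that flags an objective as triggered when the player's dialogue reaches a set line.
; BeginPlay caches the Astra player and inserts ObjectiveDialogue lines, up to the trigger index, into the Dialogue array.
; Tick polls Astra's NPCDialogueIndex and sets IsObjectiveTriggered on a match.
; The code updating the player's objective text is disconnected, and the Objective function only returns false.
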(event `self.ReceiveBeginPlay`
  (`parent.ReceiveBeginPlay`)
  (bind _asastra (cast `/Game/Astra/Astra` (`GameplayStatics.GetPlayerCharacter` 0)))
  (set `self.Astra` _asastra)
  (set `self.isObjectiveTriggered` false)
  (for (_array_element _array_index) (`self.ObjectiveDialogue`)
    (`KismetArrayLibrary.Array_Insert` (`self.Dialogue`) _array_element _array_index)
    (if (== _array_index (`self.ObjectiveDialogueIndexTrigger`))
      (break))))

(event `self.ReceiveTick`
  (params (DeltaSeconds :type "Float (single-precision)"))
  (`parent.ReceiveTick` DeltaSeconds)
  (if (== (`/Game/Astra/Astra.NPCDialogueIndex` (`self.Astra`)) (`self.ObjectiveDialogueIndexTrigger`))
    (set `self.isObjectiveTriggered` true)))

(fn `Objective`
  (returns (Success :type Boolean))
  (return false))

(fn `UserConstructionScript`
  (`parent.UserConstructionScript`))