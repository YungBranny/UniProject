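; Base Blueprint for an interactable friendly NPC that gives the player an objective through dialogue.
; On BeginPlay it caches the Astra player and inserts objective dialogue into the parent's Dialogue array, up to and including the trigger index.
; Tick flags the objective as triggered when Astra's NPC dialogue index equals that trigger.
; An overridable Objective function reports completion, returning false by default.
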(event `self.ReceiveBeginPlay`
  (`parent.ReceiveBeginPlay`)
  ;[1 1 1] Astra
  (bind _asastra (cast `/Game/Astra/Astra` (`GameplayStatics.GetPlayerCharacter` 0)))
  (set `self.Astra` _asastra)
  ;[1 1 1] Objective has not been triggered
  (set `self.isObjectiveTriggered` false)
  ;[1 1 1] Go through the objective dialogue and insert that into the dialogue array of the parent, once this is equal to the objective dialogue trigger, break the loop
  (for (_array_element _array_index) (`self.ObjectiveDialogue`)
    (`KismetArrayLibrary.Array_Insert` (`self.Dialogue`) _array_element _array_index)
    (if (== _array_index (`self.ObjectiveDialogueIndexTrigger`))
      (break))))

(event `self.ReceiveTick`
  (params (DeltaSeconds :type "Float (single-precision)"))
  (`parent.ReceiveTick` DeltaSeconds)
  ;[1 1 1] Once the dialogue index is equal to the objective index trigger, set isObjectiveTriggered to true
  (if (== (`/Game/Astra/Astra.NPCDialogueIndex` (`self.Astra`)) (`self.ObjectiveDialogueIndexTrigger`))
    (set `self.isObjectiveTriggered` true)))

(fn `Objective`
  (returns (Success :type Boolean))
  ;[1 1 1] Objective function that can be overridable, it returns a boolean to check if the objective has been completed
  (return false))

(fn `UserConstructionScript`
  (`parent.UserConstructionScript`))