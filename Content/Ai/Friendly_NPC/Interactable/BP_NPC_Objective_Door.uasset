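; Friendly NPC that gives the player a kill-count objective and opens an objective door as the reward.
; Tick shows the objective text once triggered, resets Astra's kill count once, and polls the Objective override against EnemiesToKill.
; On completion it swaps the dialogue and flashes a pop-up.
; When the player then speaks, it loops over all BP_Door_Objective actors, using a Timeline to open and re-close the door, then unlocks it.
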(event `self.ReceiveActorBeginOverlap`
  (params (OtherActor :type "Actor Object Reference"))
  (`parent.ReceiveActorBeginOverlap` OtherActor))

(event `self.ReceiveTick`
  (params (DeltaSeconds :type "Float (single-precision)"))
  (bind _w_popuptext (`/Game/Astra/Astra.W_PopUpText` (`self.Astra`)))
  (bind _w_popuptext_2 (`/Game/Astra/Astra.W_PopUpText` (`self.Astra`)))
  (`parent.ReceiveTick` DeltaSeconds)
  (`|ExecutionSequence`
    (:`then_0`
      (if (`self.isObjectiveTriggered`)
        (`|ExecutionSequence`
          (:`then_0`
            ;[1 1 1] Set current enemies killed to 0
            (`/Engine/EditorBlueprintResources/StandardMacros.DoOnce` false
              (:`Completed`
                (set `/Game/Astra/Astra.CurrentEnemiesKilled` 0 (`self.Astra`)))))
          (:`then_1`
            ;[1 1 1] Set the player objective
            (set `/Game/Astra/Astra.PlayerObjectives` (`KismetTextLibrary.Conv_StringToText` (`self.PlayerObjectiveText`)) (`self.Astra`)))
          (:`then_2`
            ;[1 1 1] If the objective has been complete, set isObjectiveComplete to true
            (bind _success (`self.Objective`))
            (if _success
              (set `self.isObjectiveComplete` true))))))
    (:`then_1`
      (if (`self.isObjectiveComplete`)
        (`|ExecutionSequence`
          (:`then_0`
            ;[1 1 1] Clear current dialogue
            (`KismetArrayLibrary.Array_Clear` (`self.Dialogue`)))
          (:`then_1`
            ;[1 1 1] Insert new dialogue for completed objective
            (`KismetArrayLibrary.Array_Insert` (`self.Dialogue`) (`|GetArrayItem` (`self.ObjectiveDialogue`) (`self.completedObjectiveDialogueIndex`))))
          (:`then_2`
            ;[1 1 1] Create pop up text to notify the player that they have completed enough enemies
            (`/Engine/EditorBlueprintResources/StandardMacros.DoOnce` false
              (:`Completed`
                (`Widget.SetVisibility` _w_popuptext_2 "Visible")
                (`TextBlock.SetText` (`/Game/GUI/W_PopUpText.T_PopUpText` _w_popuptext_2) "You've killed enough enemies!")
                (`KismetSystemLibrary.Delay` 2.0)
                (`TextBlock.SetText` (`/Game/GUI/W_PopUpText.T_PopUpText` _w_popuptext) "")
                (`Widget.SetVisibility` _w_popuptext "Hidden"))))
          (:`then_3`
            (if (`/Game/Astra/Astra.isSpeaking` (`self.Astra`))
              ;[1 1 1] Get the door linked to this bp
              (bind _outactors (`GameplayStatics.GetAllActorsOfClass` "/Game/Ai/Friendly_NPC/Interactable/BP_Door_Objective.BP_Door_Objective_C"))
              (for _array_element _outactors
                (`|ExecutionSequence`
                  (:`then_0`
                    ;[1 1 1] Set isObjectiveTriggered to false and clear the objective
                    (bind _output_get (set `self.isObjectiveTriggered` false))
                    (if (not _output_get)
                      (set `/Game/Astra/Astra.PlayerObjectives` "   " (`self.Astra`))))
                  (:`then_1`
                    ;[1 1 1] Play a sound at location (for door opening)
                    (`/Engine/EditorBlueprintResources/StandardMacros.DoOnce` false
                      (:`Completed`
                        (`GameplayStatics.PlaySoundAtLocation` "/Game/Sound/Spacedoor_Open_Cue.Spacedoor_Open_Cue" (`self.K2_GetActorLocation` _array_element) (struct) 1.0 1.0 0.0 null null null))))
                  (:`then_2`
                    ;[1 1 1] Open the door for the player, after a 3 second delay it will close
                    (bind (_direction _movedoor) (`Timeline|Timeline_0` :!label _label)
                      (:`Update`
                        (`SceneComponent.K2_SetRelativeLocation` (`/Game/Ai/Friendly_NPC/Interactable/BP_Door_Objective.Door` _array_element) (`KismetMathLibrary.VLerp` (0.0 0.0 0.0) (`/Game/Ai/Friendly_NPC/Interactable/BP_Door_Objective.TargetLocation` _array_element) _movedoor) false false))
                      (:`Finished`
                        (`KismetSystemLibrary.Delay` 3.0)
                        (goto _label :!via `Reverse`))))
                  (:`then_3`
                    ;[1 1 1] After a delay, just after the door has closed, set isLocked to false, so the player can go through the door when they want
                    (`KismetSystemLibrary.Delay` 3.5)
                    (set `/Game/Ai/Friendly_NPC/Interactable/BP_Door_Objective.isLocked` false _array_element)))))))))))

(fn `Objective`
  (returns (Success :type Boolean))
  (`parent.Objective`)
  (if (not (`self.isObjectiveComplete`))
    (return (>= (`/Game/Astra/Astra.CurrentEnemiesKilled` (`self.Astra`)) (`self.enemiesToKill`)))))

(fn `UserConstructionScript`
  (`parent.UserConstructionScript`))