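; A locked door Blueprint that opens when a player carrying enough keys walks into its trigger box.
; On overlap, it checks the character's Key count against KeyRequired, deducts that amount and plays a timeline.
; The timeline lerps the Door component's relative location from the origin to TargetLocation.
; End overlap only casts the actor, so the door never closes.
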(event `self.Box.OnComponentBeginOverlap`
  (params (OverlappedComponent :type "PrimitiveComponent Object Reference") (OtherActor :type "Actor Object Reference") (OtherComp :type "PrimitiveComponent Object Reference") (OtherBodyIndex :type Integer) (bFromSweep :type Boolean) (SweepResult :type "HitResult Structure (by ref)"))
  (bind _key_required (`self.Key required`))
  (bind _asthird_person_character_1 (cast `/Game/Astra/ThirdPersonCharacter1` OtherActor))
  (bind _key (`/Game/Astra/ThirdPersonCharacter1.Key` _asthird_person_character_1))
  (if (>= _key _key_required)
    (set `/Game/Astra/ThirdPersonCharacter1.Key` (- _key _key_required) _asthird_person_character_1)
    (bind (_direction _movedoor) (`Timeline|Timeline_0`)
      (:`Update`
        (`SceneComponent.K2_SetRelativeLocation` (`self.Door`) (`KismetMathLibrary.VLerp` (0.0 0.0 0.0) (`self.TargetLocation`) _movedoor) false false)))))

(event `self.Box.OnComponentEndOverlap`
  (params (OverlappedComponent :type "PrimitiveComponent Object Reference") (OtherActor :type "Actor Object Reference") (OtherComp :type "PrimitiveComponent Object Reference") (OtherBodyIndex :type Integer))
  (cast `/Game/Astra/ThirdPersonCharacter1` OtherActor))

(fn `UserConstructionScript`)