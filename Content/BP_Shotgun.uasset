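; Battery-powered shotgun for the Astra player character that plays a low-ammo sound when the battery is empty.
; Fire drains the battery, plays animation and camera shake, then casts ten randomly spread line traces from the ADS camera, with timeline-driven recoil.
; Hits notify the actor and AI damage sense; damageable targets take damage and bleed, others get bullet holes.
; Blood particle collisions spawn splatter decals with random frames via dynamic materials.
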(event `self.ReceiveBeginPlay`
  ;[1 1 1] Cast to astra
  (bind _asastra (cast `/Game/Astra/Astra` (`GameplayStatics.GetPlayerCharacter` 0)))
  (set `self.Astra` _asastra))

(event `OnCollideBlood`
  (params (EventName :type Name) (EmitterTime :type "Float (double-precision)") (ParticleTime :type Integer) (Location :type "Vector Structure") (Velocity :type "Vector Structure") (Direction :type "Vector Structure") (Normal :type "Vector Structure") (BoneName :type Name) (PhysMat :type "PhysicalMaterial Object Reference"))
  (bind _returnvalue (`KismetMaterialLibrary.CreateDynamicMaterialInstance` "/Game/Splatter_Decal.Splatter_Decal"))
  (`MaterialInstanceDynamic.SetScalarParameterValue` _returnvalue "Frame" (`KismetMathLibrary.Conv_IntToDouble` (`KismetMathLibrary.RandomInteger` 11)))
  (`GameplayStatics.SpawnDecalAtLocation` _returnvalue (`KismetMathLibrary.Conv_DoubleToVector` (`KismetMathLibrary.RandomFloatInRange` 10.0 30.0)) Location (`KismetMathLibrary.Conv_VectorToRotator` Normal) 15.0))

(event `/Game/GunInterface.Fire`
  (bind _returnvalue (`GameplayStatics.GetPlayerCharacter` 0))
  (bind _astra (`self.Astra`))
  (bind _adscamera (`/Game/Astra/Astra.ADSCamera` (`self.Astra`)))
  (bind _returnvalue_2 (`SceneComponent.K2_GetComponentLocation` _adscamera))
  (set `/Game/Astra/Astra.Decrease Battery Amount` 10.0 _astra)
  (if (<= (`/Game/Astra/Astra.CurrentBattery` _astra) 0.0)
    (`GameplayStatics.PlaySoundAtLocation` "/Game/Sound/lowammo_01.lowammo_01" (`self.K2_GetActorLocation`) (struct) 1.0 1.0 0.0 null null null)
    (else
      (`/Game/Astra/Astra.Battery Decrease Bullet` (`self.Astra`))
      (`SkeletalMeshComponent.PlayAnimation` (`self.SkeletalMesh`) "/Game/SciFiWeapLight/Weapons/Anims/Fire_Shotgun_W.Fire_Shotgun_W" false)
      (`GameplayStatics.PlayWorldCameraShake` "/Game/ShotGun_Shake.ShotGun_Shake_C" _returnvalue_2 0.0 500.0)
      (for _ (range 10)
        (bind (_outhit _returnvalue_3) (`KismetSystemLibrary.LineTraceSingle` :`Start` _returnvalue_2 :`End` (`KismetMathLibrary.MakeVector` (+ (.x (+ _returnvalue_2 (* (`SceneComponent.GetForwardVector` _adscamera) 1000.0))) (`KismetMathLibrary.RandomFloatInRange` -200.0 200.0)) (+ (.y (+ _returnvalue_2 (* (`SceneComponent.GetForwardVector` _adscamera) 1000.0))) (`KismetMathLibrary.RandomFloatInRange` -200.0 200.0)) (+ (.z (+ _returnvalue_2 (* (`SceneComponent.GetForwardVector` _adscamera) 1000.0))) (`KismetMathLibrary.RandomFloatInRange` -200.0 200.0))) :`TraceChannel` "TraceTypeQuery1" :`DrawTime` 1000.0))
        (`|ExecutionSequence`
          (:`then_0`
            (if _returnvalue_3
              (bind (_bblockinghit _binitialoverlap _time _distance _location _impactpoint _normal _impactnormal _physmat _hitactor _hitcomponent _hitbonename _hititem _faceindex _tracestart) (`GameplayStatics.BreakHitResult` _outhit))
              (message `/Game/Ai/BossNPC/CollisionDetection.OnHit` _hitactor _impactpoint)
              (`/Engine/EditorBlueprintResources/StandardMacros.IsValid` _hitactor
                (:`Is Valid`
                  _)
                (:`Is Not Valid`
                  _))
              (`AISense_Damage.ReportDamageEvent` _hitactor (`GameplayStatics.GetPlayerCharacter` 0) 0.0 _tracestart)
              (if (`Actor.bCanBeDamaged` _hitactor)
                (bind _returnvalue_4 (`KismetMathLibrary.MakeRotFromX` _normal))
                (`GameplayStatics.SpawnEmitterAtLocation` "/Game/StarterContent/Particles/Blood.Blood" _impactpoint _returnvalue_4)
                (bind _returnvalue_5 (`GameplayStatics.SpawnEmitterAtLocation` "/Game/P_Splatter.P_Splatter" _impactpoint _returnvalue_4))
                (add `ParticleSystemComponent.OnParticleCollide` _returnvalue_5 (delegate `OnCollideBlood`))
                (`GameplayStatics.ApplyDamage` _hitactor 7.0 null (`GameplayStatics.GetPlayerCharacter` 0))
                (else
                  (`GameplayStatics.SpawnEmitterAtLocation` "/Game/SciFiWeapLight/FX/Particles/P_Impact_Metal_Medium_Dark.P_Impact_Metal_Medium_Dark" _impactpoint _returnvalue_4)
                  (bind _returnvalue_6 (`GameplayStatics.SpawnDecalAtLocation` "/Game/Decal_Bullet_Hole.Decal_Bullet_Hole" (10.0 10.0 10.0) _impactpoint _returnvalue_4 10.0))
                  (`SceneComponent.K2_AttachToComponent` _returnvalue_6 _hitcomponent "None" "KeepWorld" "KeepWorld" "KeepWorld" true)))))
          (:`then_1`
            (`Timeline|Timeline_0`
              (:`Update`
                (`Pawn.AddControllerYawInput` _returnvalue (`KismetMathLibrary.RandomFloatInRange` -0.15 0.15))
                (`Pawn.AddControllerPitchInput` _returnvalue (`KismetMathLibrary.RandomFloatInRange` -1.5 -1.5))))))))))

(fn `UserConstructionScript`)