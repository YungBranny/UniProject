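; Charging station that refills the battery of the player character, Astra, while Interact is held inside its sphere, drawing on the station's own limited charge.
; Sphere overlap toggles the actor's input, and pressing Interact starts a looping timer that drains the station, updates its Charge material parameter and adds to the player's battery.
; Release, an empty station or a full player battery clears the timer and plays the station's montage in reverse.
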(event `InputAction|Interact`
  (params (Key :type "Key Structure"))
  (bind _playercharacter (`self.PlayerCharacter`))
  ;[1 1 1] The Charging Station only depletes if Charge is greater than 0.
  (:`Pressed`
    (if (> (`self.BatteryCharge`) 0.0)
      (if (<= (`/Game/Astra/Astra.MaxBattery` _playercharacter) (`/Game/Astra/Astra.CurrentBattery` _playercharacter))
        (`self.EndDepletion`)
        (else
          (`self.StartDepletion`)))))
  (:`Released`
    (`self.EndDepletion`)))

(event `self.Sphere.OnComponentBeginOverlap`
  (params (OverlappedComponent :type "PrimitiveComponent Object Reference") (OtherActor :type "Actor Object Reference") (OtherComp :type "PrimitiveComponent Object Reference") (OtherBodyIndex :type Integer) (bFromSweep :type Boolean) (SweepResult :type "HitResult Structure (by ref)"))
  ;[1 1 1] The Player Character is able to use Health Station when inside it's radius, otherwise the Game disables input.
  (bind _asastra (cast `/Game/Astra/Astra` OtherActor))
  (set `self.PlayerCharacter` _asastra)
  (`self.EnableInput` (`GameplayStatics.GetPlayerController` 0)))

(event `self.Sphere.OnComponentEndOverlap`
  (params (OverlappedComponent :type "PrimitiveComponent Object Reference") (OtherActor :type "Actor Object Reference") (OtherComp :type "PrimitiveComponent Object Reference") (OtherBodyIndex :type Integer))
  ;[1 1 1] The Player Character is able to use Health Station when inside it's radius, otherwise the Game disables input.
  (cast `/Game/Astra/Astra` OtherActor)
  (`self.DisableInput` (`GameplayStatics.GetPlayerController` 0)))

(event `StartDepletion`
  ;[1 1 1] Make sure charge doesn't go below 0.
  (bind _returnvalue (`KismetSystemLibrary.K2_SetTimerDelegate` (delegate `Decharge`) 0.1 true)) ; Decharge every 0.1 seconds.
  (set `self.DechargeTimer` _returnvalue)
  (`|PlayMontage` (`self.SkeletalMesh`) "/Game/HealthSystem/ChargingStation/Animations/AM_ChargingStationMontage.AM_ChargingStationMontage"))

(event `Decharge`
  (bind _playercharacter (`self.PlayerCharacter`))
  (bind _playercharacter_2 (`self.PlayerCharacter`))
  (bind _returnvalue (`KismetMathLibrary.FClamp` (- (`self.BatteryCharge`) 0.01) 0.0 1.0))
  ;[1 1 1] Make sure charge doesn't go below 0.
  (`MeshComponent.SetScalarParameterValueOnMaterials` (`self.SkeletalMesh`) "Charge" _returnvalue)
  (bind _output_get (set `self.BatteryCharge` _returnvalue))
  (if (<= _output_get 0.0)
    (`self.EndDepletion`) ; If it goes below 0, end depletion.
    (else
      (set `/Game/Astra/Astra.CurrentBattery` (+ (`/Game/Astra/Astra.CurrentBattery` _playercharacter) (`self.BatteryIncreaseAmount`)) _playercharacter)
      (if (<= (`/Game/Astra/Astra.MaxBattery` _playercharacter_2) (`/Game/Astra/Astra.CurrentBattery` _playercharacter_2))
        (`self.EndDepletion`)))))

(event `EndDepletion`
  ;[1 1 1] Stops continuous loop.
  (`KismetSystemLibrary.K2_ClearAndInvalidateTimerHandle` (`self.DechargeTimer`))
  (`|PlayMontage` (`self.SkeletalMesh`) "/Game/HealthSystem/ChargingStation/Animations/AM_ChargingStationMontage.AM_ChargingStationMontage" -1.0 0.3) ; Plays Animation.
)

(fn `UserConstructionScript`)