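; Sliding door actor that opens when the Astra character enters its box trigger and closes when it leaves.
; A timeline plays or reverses on overlap, lerping the door's relative location from zero to TargetLocation.
; A DoOnce on the timeline update plays the open sound at the door, resetting when the timeline finishes, so the same cue also sounds on a close from fully open.
; Damage is disabled at BeginPlay.
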(event `self.ReceiveBeginPlay`
  (set `self.bCanBeDamaged` false))

(event `self.Box.OnComponentBeginOverlap`
  (params (OverlappedComponent :type "PrimitiveComponent Object Reference") (OtherActor :type "Actor Object Reference") (OtherComp :type "PrimitiveComponent Object Reference") (OtherBodyIndex :type Integer) (bFromSweep :type Boolean) (SweepResult :type "HitResult Structure (by ref)"))
  ;[1 1 1] Door opens and closes when player enters and exits box trigger
  (cast `/Game/Astra/Astra` OtherActor)
  (bind (_direction _movedoor) (`Timeline|MoveDoor` :!label _label)
    (:`Update`
      (`|ExecutionSequence`
        (:`then_0`
          (`/Engine/EditorBlueprintResources/StandardMacros.DoOnce` false :!label _label_2
            (:`Completed`
              (`GameplayStatics.PlaySoundAtLocation` "/Game/Sound/Spacedoor_Open_Cue.Spacedoor_Open_Cue" (`SceneComponent.K2_GetComponentLocation` (`self.Door`)) (struct) 1.0 1.0 0.0 null null null))))
        (:`then_1`
          (`SceneComponent.K2_SetRelativeLocation` (`self.Door`) (`KismetMathLibrary.VLerp` (0.0 0.0 0.0) (`self.TargetLocation`) _movedoor) false false))))
    (:`Finished`
      (goto _label_2 :!via `Reset`))))

(event `self.Box.OnComponentEndOverlap`
  (params (OverlappedComponent :type "PrimitiveComponent Object Reference") (OtherActor :type "Actor Object Reference") (OtherComp :type "PrimitiveComponent Object Reference") (OtherBodyIndex :type Integer))
  ;[1 1 1] Door opens and closes when player enters and exits box trigger
  (cast `/Game/Astra/Astra` OtherActor)
  (goto _label :!via `Reverse`))

(fn `UserConstructionScript`)