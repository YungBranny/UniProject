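; Timed door Blueprint, named for the final room, that slides open once after a countdown started by the Astra character.
; Entering or leaving the box trigger calls TimerTick, which increments a counter and repeats through a one-second RetriggerableDelay loop; leaving does not stop it.
; At the unlock threshold, a DoOnce-guarded Timeline lerps the door's relative location to its target, with no closing logic.
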(event `self.ReceiveBeginPlay`
  (set `self.bCanBeDamaged` false)
  (`SceneComponent.K2_SetRelativeLocation` (`self.Box`) (`self.BoxTriggerLocation`) false false))

(event `self.Box.OnComponentBeginOverlap`
  (params (OverlappedComponent :type "PrimitiveComponent Object Reference") (OtherActor :type "Actor Object Reference") (OtherComp :type "PrimitiveComponent Object Reference") (OtherBodyIndex :type Integer) (bFromSweep :type Boolean) (SweepResult :type "HitResult Structure (by ref)"))
  ;[1 1 1] Door opens and closes when player enters and exits box trigger
  (cast `/Game/Astra/Astra` OtherActor)
  (`self.TimerTick` :!label _label))

(event `self.Box.OnComponentEndOverlap`
  (params (OverlappedComponent :type "PrimitiveComponent Object Reference") (OtherActor :type "Actor Object Reference") (OtherComp :type "PrimitiveComponent Object Reference") (OtherBodyIndex :type Integer))
  ;[1 1 1] Door opens and closes when player enters and exits box trigger
  (cast `/Game/Astra/Astra` OtherActor)
  (goto _label))

(event `TimerTick`
  (bind _output_get (set `self.Timer` (+ (`self.Timer`) 1) :!label _label_2))
  (if (>= _output_get (`self.TimeForDoorToUnlock`))
    (`self.Door Open`)
    (else
      (`KismetSystemLibrary.RetriggerableDelay` 1.0)
      (goto _label_2))))

(event `Door Open`
  (`/Engine/EditorBlueprintResources/StandardMacros.DoOnce` false
    (:`Completed`
      (bind (_direction _movedoor) (`Timeline|Timeline_0` :!via `PlayFromStart`)
        (:`Update`
          (`SceneComponent.K2_SetRelativeLocation` (`self.Door`) (`KismetMathLibrary.VLerp` (0.0 0.0 0.0) (`self.TargetLocation`) _movedoor) false false))))))

(fn `UserConstructionScript`)