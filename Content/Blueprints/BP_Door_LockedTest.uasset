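; BP_Door_LockedTest is a locked door that slides open when an Astra player with enough keys enters its trigger box.
; On overlap, it compares KeyCount to KeyRequired, subtracts that cost from the player and plays a timeline that lerps the door's relative location from zero to TargetLocation.
; Nothing closes the door or records it as opened, so each qualifying re-entry deducts keys again.
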(event `self.Box.OnComponentBeginOverlap`
  (params (OverlappedComponent :type "PrimitiveComponent Object Reference") (OtherActor :type "Actor Object Reference") (OtherComp :type "PrimitiveComponent Object Reference") (OtherBodyIndex :type Integer) (bFromSweep :type Boolean) (SweepResult :type "HitResult Structure (by ref)"))
  (bind _key_required (`self.Key required`))
  ;[1 1 1] Removes key from player so the next locked door will require a new key
  (bind _asastra (cast `/Game/Astra/Astra` OtherActor))
  (bind _keycount (`/Game/Astra/Astra.KeyCount` _asastra))
  (if (>= _keycount _key_required)
    (set `/Game/Astra/Astra.KeyCount` (- _keycount _key_required) _asastra)
    ;[1 1 1] Opens the door if the player has a key
    (bind (_direction _movedoor) (`Timeline|Timeline_0`)
      (:`Update`
        (`SceneComponent.K2_SetRelativeLocation` (`self.Door`) (`KismetMathLibrary.VLerp` (0.0 0.0 0.0) (`self.TargetLocation`) _movedoor) false false)))))

(event `self.Box.OnComponentEndOverlap`
  (params (OverlappedComponent :type "PrimitiveComponent Object Reference") (OtherActor :type "Actor Object Reference") (OtherComp :type "PrimitiveComponent Object Reference") (OtherBodyIndex :type Integer))
  (cast `/Game/Astra/Astra` OtherActor))

(fn `UserConstructionScript`)