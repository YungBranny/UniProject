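; A key-locked door that slides open when the Astra character enters its trigger box carrying enough keys.
; On overlap it deducts the required keys, then a timeline lerps the door's relative location to a target and clears the locked flag, with no closing logic.
; A second trigger shows a hint text only while the door is locked and the player lacks keys.
; The text rotates every tick to face the player.
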(event `self.ReceiveBeginPlay`
  ;[1 0 1] Set isDoorLocked to True
  (set `self.isDoorLocked` true)
  ;[1 0 1] Set the InteractionText to not visible
  (`SceneComponent.SetVisibility` (`self.InteractionText`) false false))

(event `self.ReceiveTick`
  (params (DeltaSeconds :type "Float (single-precision)"))
  (bind _interactiontext (`self.InteractionText`))
  ;[1 0 1] Set the rotation of theInteractionText to facing the player
  (`SceneComponent.K2_SetWorldRotation` _interactiontext (`KismetMathLibrary.FindLookAtRotation` (`SceneComponent.K2_GetComponentLocation` _interactiontext) (`self.K2_GetActorLocation` (`GameplayStatics.GetPlayerPawn` 0))) false false))

(event `self.Box.OnComponentBeginOverlap`
  (params (OverlappedComponent :type "PrimitiveComponent Object Reference") (OtherActor :type "Actor Object Reference") (OtherComp :type "PrimitiveComponent Object Reference") (OtherBodyIndex :type Integer) (bFromSweep :type Boolean) (SweepResult :type "HitResult Structure (by ref)"))
  (bind _key_required (`self.Key required`))
  (bind _asastra (cast `/Game/Astra/Astra` OtherActor))
  (bind _keycount (`/Game/Astra/Astra.KeyCount` _asastra))
  (if (and (>= _keycount _key_required) (== (`self.isDoorLocked`) true))
    (set `/Game/Astra/Astra.KeyCount` (- _keycount _key_required) _asastra)
    (bind (_direction _movedoor) (`Timeline|Timeline_0`)
      (:`Update`
        (`SceneComponent.K2_SetRelativeLocation` (`self.Door`) (`KismetMathLibrary.VLerp` (0.0 0.0 0.0) (`self.TargetLocation`) _movedoor) false false)
        (set `self.isDoorLocked` false)))))

(event `self.Box.OnComponentEndOverlap`
  (params (OverlappedComponent :type "PrimitiveComponent Object Reference") (OtherActor :type "Actor Object Reference") (OtherComp :type "PrimitiveComponent Object Reference") (OtherBodyIndex :type Integer))
  (cast `/Game/Astra/Astra` OtherActor))

(event `self.InteractText.OnComponentBeginOverlap`
  (params (OverlappedComponent :type "PrimitiveComponent Object Reference") (OtherActor :type "Actor Object Reference") (OtherComp :type "PrimitiveComponent Object Reference") (OtherBodyIndex :type Integer) (bFromSweep :type Boolean) (SweepResult :type "HitResult Structure (by ref)"))
  (bind _interactiontext (`self.InteractionText`))
  ;[1 0 1] If the player is in the InteractText box collision, check to see if the InteractionText should be visible or not.
  (bind _asastra (cast `/Game/Astra/Astra` OtherActor))
  (if (or (>= (`/Game/Astra/Astra.KeyCount` _asastra) (`self.Key required`)) (== (`self.isDoorLocked`) false))
    (`SceneComponent.SetVisibility` _interactiontext false false) ; Set the InteractionText to not be visible
    (else
      (`SceneComponent.SetVisibility` _interactiontext true false) ; Set the InteractionText to be visible
    )))

(event `self.InteractText.OnComponentEndOverlap`
  (params (OverlappedComponent :type "PrimitiveComponent Object Reference") (OtherActor :type "Actor Object Reference") (OtherComp :type "PrimitiveComponent Object Reference") (OtherBodyIndex :type Integer))
  ;[1 0 1] If the player is not in the InteractText box collision, set the InteractionText to not be visible
  (cast `/Game/Astra/Astra` OtherActor)
  (`SceneComponent.SetVisibility` (`self.InteractionText`) false false))

(fn `UserConstructionScript`)