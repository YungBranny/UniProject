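; Explosive barrel actor that blows up when shot, through its OnHit event.
; OnHit plays explosion sound and particles, shakes the camera around Astra's ADS camera, projects a burn decal via a downward trace, and flashes a point light.
; After the flash it spawns an Aoe_Barrel damage collider, enables physics and applies radius damage to fracture the drum mesh, then destroys itself after a delay.
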(event `self.ReceiveBeginPlay`
  (set `self.bCanBeDamaged` false))

(event `/Game/Ai/BossNPC/CollisionDetection.OnHit`
  (params (HitLocation :type "Vector Structure"))
  (bind _sm_waterdrum_dm (`self.SM_WaterDrum_DM`))
  ;[1 1 1] When the player shoots a barrel it blows up and does this
  (bind _asastra (cast `/Game/Astra/Astra` (`GameplayStatics.GetPlayerCharacter` 0)))
  (`GameplayStatics.PlaySoundAtLocation` "/Game/StarterContent/Audio/Explosion01.Explosion01" HitLocation (struct) 1.0 1.0 0.0 null null null)
  (`GameplayStatics.SpawnEmitterAtLocation` "/Game/StarterContent/Particles/P_Explosion.P_Explosion" HitLocation (struct) (5.0 5.0 5.0))
  (`GameplayStatics.PlayWorldCameraShake` "/Game/Blueprints/Barrel_Shake.Barrel_Shake_C" (`SceneComponent.K2_GetComponentLocation` (`/Game/Astra/Astra.ADSCamera` _asastra)) 1000.0 1000.0)
  (bind _outhit (`KismetSystemLibrary.LineTraceSingle` HitLocation (- HitLocation (0.0 0.0 100.0)) "TraceTypeQuery1"))
  (bind (_bblockinghit _binitialoverlap _time _distance _location _impactpoint _normal) (`GameplayStatics.BreakHitResult` _outhit))
  (`GameplayStatics.SpawnDecalAtLocation` "/Game/Materials/Burn_Decal.Burn_Decal" (`KismetMathLibrary.Conv_DoubleToVector` (`KismetMathLibrary.RandomFloatInRange` 90.0 125.0)) _impactpoint (`KismetMathLibrary.MakeRotFromX` _normal) 10.0)
  (`SceneComponent.SetVisibility` (`self.PointLight`) true false)
  (`KismetSystemLibrary.Delay` 0.3)
  (`SceneComponent.SetVisibility` (`self.PointLight`) false false)
  ;;[1 1 1] Spawns damage collider
  (`|SpawnActorFromClass` "/Game/Blueprints/Aoe_Barrel.Aoe_Barrel_C" (`KismetMathLibrary.Conv_VectorToTransform` (`self.K2_GetActorLocation`)) "Undefined" "OverrideRootScale" null null)
  ;;[1 1 1] Applies the force to explode the barrel
  (`PrimitiveComponent.SetSimulatePhysics` _sm_waterdrum_dm true)
  (`DestructibleComponent.ApplyRadiusDamage` _sm_waterdrum_dm 40.0 HitLocation 40.0 10000.0 false)
  (`KismetSystemLibrary.Delay` 3.0)
  (`self.K2_DestroyActor`))

(fn `UserConstructionScript`)