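; Cutscene trigger actor that plays a Level Sequence the first time the player character enters its box.
; BeginPlay creates and stores the sequence player, and the box overlap passes through a DoOnce to disable player input and start playback.
; A one-shot timer set to the sequence's duration re-enables input, rather than binding to the player's finished event.
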(event `self.ReceiveBeginPlay`
  (bind (_outactor _returnvalue) (`LevelSequencePlayer.CreateLevelSequencePlayer` null))
  (set `self.Scene` _returnvalue))

(event `self.Box.OnComponentBeginOverlap`
  (params (OverlappedComponent :type "PrimitiveComponent Object Reference") (OtherActor :type "Actor Object Reference") (OtherComp :type "PrimitiveComponent Object Reference") (OtherBodyIndex :type Integer) (bFromSweep :type Boolean) (SweepResult :type "HitResult Structure (by ref)"))
  (bind _returnvalue (`GameplayStatics.GetPlayerCharacter` 0))
  (bind _scene (`self.Scene`))
  (if (== OtherActor _returnvalue)
    (`/Engine/EditorBlueprintResources/StandardMacros.DoOnce` false
      (:`Completed`
        (`self.DisableInput` _returnvalue (`GameplayStatics.GetPlayerController` 0))
        (`MovieSceneSequencePlayer.Play` _scene)
        (`KismetSystemLibrary.K2_SetTimerDelegate` (delegate `EnableMovement`) (`TimeManagementBlueprintLibrary.Conv_QualifiedFrameTimeToSeconds` (`MovieSceneSequencePlayer.GetDuration` _scene)))))))

(event `EnableMovement`
  (`self.EnableInput` (`GameplayStatics.GetPlayerCharacter` 0) (`GameplayStatics.GetPlayerController` 0)))

(fn `UserConstructionScript`)