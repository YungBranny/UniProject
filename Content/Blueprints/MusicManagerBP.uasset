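; MusicManagerBP is a music manager that switches between background tracks at runtime.
; On BeginPlay it creates a 2D sound for each entry in SoundList, starts them all playing muted, then raises the starting track to MusicVolume.
; ChangeMusic mutes the current track and unmutes the chosen one by index, so switches are instant volume swaps between simultaneously playing tracks, without restarts or crossfades.
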(event `Change Music`
  (params (SoundToPlay :type Integer))
  (bind _output (`|GetArrayItem` (`self.SoundReference`) SoundToPlay))
  (`AudioComponent.SetVolumeMultiplier` (`self.CurrentSoundReference`) 0.0)
  (`AudioComponent.SetVolumeMultiplier` _output (`self.MusicVolume`))
  (set `self.CurrentSoundReference` _output))

(event `self.ReceiveBeginPlay`
  (bind _output (`|GetArrayItem` (`self.SoundReference`) (`self.SoundToPlayOnStart`)))
  (for _array_element (`self.SoundList`)
    (bind _returnvalue (`GameplayStatics.CreateSound2D` _array_element 1.0 1.0 0.0 null))
    (`KismetArrayLibrary.Array_Add` (`self.SoundReference`) _returnvalue)
    (`AudioComponent.SetVolumeMultiplier` _returnvalue 0.0)
    (`AudioComponent.Play` _returnvalue 0.0))
  (`AudioComponent.SetVolumeMultiplier` _output (`self.MusicVolume`))
  (set `self.CurrentSoundReference` _output))

(fn `UserConstructionScript`)