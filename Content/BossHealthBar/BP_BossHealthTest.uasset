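; BP_BossHealthTest is a test Blueprint that damages the player on overlap and displays a boss health bar.
; When Astra begins overlapping its Box, it subtracts a random amount from her CurrentHealth.
; Every Tick, it casts its Widget component's object to WBP_BossHealthUI and sets the progress bar from BossHealth on a 100-point scale.
; BossHealth is never changed in these graphs, so the overlap damage does not affect the bar.
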(event `self.Box.OnComponentBeginOverlap`
  (params (OverlappedComponent :type "PrimitiveComponent Object Reference") (OtherActor :type "Actor Object Reference") (OtherComp :type "PrimitiveComponent Object Reference") (OtherBodyIndex :type Integer) (bFromSweep :type Boolean) (SweepResult :type "HitResult Structure (by ref)"))
  ;[1 1 1] This Blueprint was used by me (Mia) as a Player Character test for the Player Health. Once Player Character overlaps the Damage Box, the Damage Box deals damage to the Player Character in between the range of 10 to 25. and takes away that much from the Current Health of the Player Character and sets it.
  (bind _asastra (cast `/Game/Astra/Astra` OtherActor)) ; Makes sure it only applies to our Player Character.
  (set `/Game/Astra/Astra.CurrentHealth` (- (`/Game/Astra/Astra.CurrentHealth` _asastra) (`KismetMathLibrary.RandomFloatInRange` 10.0 25.0)) _asastra))

(event `self.ReceiveTick`
  (params (DeltaSeconds :type "Float (single-precision)"))
  (bind _aswbp_boss_health_ui (cast `/Game/BossHealthBar/WBP_BossHealthUI` (`WidgetComponent.GetUserWidgetObject` (`self.Widget`))))
  (`ProgressBar.SetPercent` (`/Game/BossHealthBar/WBP_BossHealthUI.ProgressBar_82` _aswbp_boss_health_ui) (/ (`self.BossHealth`) 100.0)))

(fn `UserConstructionScript`)