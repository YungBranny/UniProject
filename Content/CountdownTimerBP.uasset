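; Countdown timer actor that, once ThirdPersonCharacter1 overlaps its trigger, counts down on a text component to a game over screen.
; Tick and the overlap share one chain, gated by casting the last overlapping actor, so a one-second Delay repeats as the countdown clock.
; Each step at zero or below adds a new GameOver widget and shows the mouse cursor, as nothing stops the loop.
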(event `self.ReceiveTick`
  (params (DeltaSeconds :type "Float (single-precision)"))
  (cast `/Game/Astra/ThirdPersonCharacter1` (stale `self.CountdownTrigger.OnComponentBeginOverlap` OtherActor) :!label _label)
  (`KismetSystemLibrary.Delay` 1.0)
  (set `self.TimeValue` (- (`self.TimeValue`) 1))
  (`TextRenderComponent.K2_SetText` (`self.Countdown`) (`KismetTextLibrary.Conv_IntToText` (`self.TimeValue`)))
  (if (<= (`self.TimeValue`) 0)
    (bind _returnvalue (`|CreateWidget` "/Game/GameOverScreen/GameOver.GameOver_C"))
    (`UserWidget.AddToViewport` _returnvalue 0)
    (bind _asplayer_controller (cast `PlayerController` (`GameplayStatics.GetPlayerController` 0)))
    (set `PlayerController.bShowMouseCursor` true _asplayer_controller)))

(event `self.CountdownTrigger.OnComponentBeginOverlap`
  (params (OverlappedComponent :type "PrimitiveComponent Object Reference") (OtherActor :type "Actor Object Reference") (OtherComp :type "PrimitiveComponent Object Reference") (OtherBodyIndex :type Integer) (bFromSweep :type Boolean) (SweepResult :type "HitResult Structure (by ref)"))
  (goto _label))

(fn `UserConstructionScript`)