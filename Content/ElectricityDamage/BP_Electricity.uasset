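; BP_Electricity is an electrical hazard that repeatedly damages the Astra character while it stays inside a collision box.
; Entering the box shows a damage widget and starts a one-second Delay loop that directly subtracts from CurrentHealth.
; When health runs out, it calls PlayerDeath on player character 0.
; Leaving clears the InFireRadius flag that keeps the loop running, but does not remove the widget.
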(event `self.BoxCollision.OnComponentBeginOverlap`
  (params (OverlappedComponent :type "PrimitiveComponent Object Reference") (OtherActor :type "Actor Object Reference") (OtherComp :type "PrimitiveComponent Object Reference") (OtherBodyIndex :type Integer) (bFromSweep :type Boolean) (SweepResult :type "HitResult Structure (by ref)"))
  (bind _asastra (cast `/Game/Astra/Astra` OtherActor))
  (set `self.InFireRadius` true)
  (bind _returnvalue (`|CreateWidget` "/Game/DamageIndicator/WBP_DamageWidget.WBP_DamageWidget_C"))
  (`UserWidget.AddToViewport` _returnvalue 0)
  (bind _output_get (set `/Game/Astra/Astra.CurrentHealth` (- (`/Game/Astra/Astra.CurrentHealth` _asastra) 5.0) _asastra :!label _label))
  (if (<= _output_get 0.0)
    (bind _asastra_2 (cast `/Game/Astra/Astra` (`GameplayStatics.GetPlayerCharacter` 0)))
    (`/Game/Astra/Astra.PlayerDeath` _asastra_2)
    (else
      (`KismetSystemLibrary.Delay` 1.0)
      (if (`self.InFireRadius`)
        (goto _label)))))

(event `self.BoxCollision.OnComponentEndOverlap`
  (params (OverlappedComponent :type "PrimitiveComponent Object Reference") (OtherActor :type "Actor Object Reference") (OtherComp :type "PrimitiveComponent Object Reference") (OtherBodyIndex :type Integer))
  (cast `/Game/Astra/Astra` OtherActor)
  (set `self.InFireRadius` false))

(fn `UserConstructionScript`)