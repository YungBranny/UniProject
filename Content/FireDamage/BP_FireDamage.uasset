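; BP_FireDamage is a fire hazard that repeatedly damages the Astra player while they stand inside its BoxCollision.
; Overlap begin sets InFireRadius and starts a one-second Delay loop that lowers Armour, also reducing CurrentHealth once Armour is depleted.
; Each hit adds a new armour or health damage widget to the viewport.
; End overlap clears the flag to stop the loop, and zero health calls PlayerDeath.
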(event `self.BoxCollision.OnComponentBeginOverlap`
  (params (OverlappedComponent :type "PrimitiveComponent Object Reference") (OtherActor :type "Actor Object Reference") (OtherComp :type "PrimitiveComponent Object Reference") (OtherBodyIndex :type Integer) (bFromSweep :type Boolean) (SweepResult :type "HitResult Structure (by ref)"))
  ;[1 1 1] When Player collides with BoxCollision and is inside the Fire radius, it damages the Armour and then goes onto the Health once Armour is equal to or below 0. Once Health reaches 0, it calls 'Death'. If not, there is a delay when Player stands in Fire and they slowly take damage.
  (bind _asastra (cast `/Game/Astra/Astra` OtherActor))
  (set `self.InFireRadius` true)
  (bind _output_get (set `/Game/Astra/Astra.Armour` (- (`/Game/Astra/Astra.Armour` _asastra) 5.0) _asastra :!label _label))
  (if (<= _output_get 0.0)
    (bind _returnvalue (`|CreateWidget` "/Game/DamageIndicator/UI/DamageUI/WBP_DamageWidget.WBP_DamageWidget_C"))
    (`UserWidget.AddToViewport` _returnvalue 0)
    (bind _output_get_2 (set `/Game/Astra/Astra.CurrentHealth` (- (`/Game/Astra/Astra.CurrentHealth` _asastra) 5.0) _asastra))
    (if (<= _output_get_2 0.0)
      (bind _asastra_2 (cast `/Game/Astra/Astra` (`GameplayStatics.GetPlayerCharacter` 0)))
      (`/Game/Astra/Astra.PlayerDeath` _asastra_2)
      (else
        (`KismetSystemLibrary.Delay` 1.0 :!label _label_2)
        (if (`self.InFireRadius`)
          (goto _label))))
    (else
      (bind _returnvalue_2 (`|CreateWidget` "/Game/DamageIndicator/UI/ArmourDamageUI/WBP_ArmourDamageWidget.WBP_ArmourDamageWidget_C"))
      (`UserWidget.AddToViewport` _returnvalue_2 0)
      (goto _label_2))))

(event `self.BoxCollision.OnComponentEndOverlap`
  (params (OverlappedComponent :type "PrimitiveComponent Object Reference") (OtherActor :type "Actor Object Reference") (OtherComp :type "PrimitiveComponent Object Reference") (OtherBodyIndex :type Integer))
  ;[1 1 1] Stop taking Fire Damage once outside its radius.
  (cast `/Game/Astra/Astra` OtherActor)
  (set `self.InFireRadius` false))

(fn `UserConstructionScript`)