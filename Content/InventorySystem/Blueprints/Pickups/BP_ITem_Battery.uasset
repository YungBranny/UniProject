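; Battery inventory item that recharges the gun battery of the player's Astra character when used.
; The UseItem interface event adds the item's ItemStructure value to CurrentBattery, clamped to MaxBattery, plays a sound and decrements the inventory size.
; A separate Use override calls its parent, then adds the same value without clamping, sound or inventory update, and returns true.
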(event `/Game/InventorySystem/Interface_Pickups.UseItem`
  (bind (_itemstructure_name _itemstructure_icon _itemstructure_description _itemstructure_value) (break `/Game/InventorySystem/Structures/Struct_Item` (`self.ItemStructure`)))
  ;[1 1 1] Interface - Using the item - When called increase the battery of the players gun.
  (bind _asastra (cast `/Game/Astra/Astra` (`GameplayStatics.GetPlayerCharacter` 0)))
  (set `/Game/Astra/Astra.CurrentBattery` (`KismetMathLibrary.FClamp` (+ (`/Game/Astra/Astra.CurrentBattery` _asastra) _itemstructure_value) 0.0 (`/Game/Astra/Astra.MaxBattery` _asastra)) _asastra)
  (`GameplayStatics.PlaySoundAtLocation` "/Game/Sound/PickUps/UseItem_Cue.UseItem_Cue" (`self.K2_GetActorLocation`) (struct) 1.0 1.0 0.0 null null null)
  ;;[1 1 1] Decrease players inventory size when the item is used
  (set `/Game/Astra/Astra.iCurrentInventorySize` (- (`/Game/Astra/Astra.iCurrentInventorySize` _asastra) 1) _asastra))

(fn `Use`
  (returns (Success :type Boolean))
  (bind (_itemstructure_name _itemstructure_icon _itemstructure_description _itemstructure_value) (break `/Game/InventorySystem/Structures/Struct_Item` (`self.ItemStructure`)))
  (`parent.Use`)
  (bind _asastra (cast `/Game/Astra/Astra` (`GameplayStatics.GetPlayerCharacter` 0)))
  (set `/Game/Astra/Astra.CurrentBattery` (+ (`/Game/Astra/Astra.CurrentBattery` _asastra) _itemstructure_value) _asastra)
  (return true))

(fn `UserConstructionScript`
  (`parent.UserConstructionScript`))