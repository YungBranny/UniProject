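; Health item for the inventory system that raises the player character's CurrentHealth when used.
; The Use override calls its parent, casts player 0's character to ThirdPersonCharacter1, adds the item structure's Value to health with no clamp, and returns true.
; A UseItem event in the event graph repeats the same addition through the player pawn, alongside an unconnected call to Use.
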(event `self.ReceiveEndPlay`
  (params (EndPlayReason :type "EEndPlayReason Enum" :default "Destroyed")))

(event `/Game/InventorySystem/Interface_Pickups.UseItem`
  (bind (_itemstructure_name _itemstructure_icon _itemstructure_description _itemstructure_value) (break `/Game/InventorySystem/Structures/Struct_Item` (`self.ItemStructure`)))
  (bind _asthird_person_character_1 (cast `/Game/Astra/ThirdPersonCharacter1` (`GameplayStatics.GetPlayerPawn` 0)))
  (set `/Game/Astra/ThirdPersonCharacter1.CurrentHealth` (+ (`/Game/Astra/ThirdPersonCharacter1.CurrentHealth` _asthird_person_character_1) _itemstructure_value) _asthird_person_character_1))

(fn `Use`
  (returns (Success :type Boolean))
  (bind (_itemstructure_name _itemstructure_icon _itemstructure_description _itemstructure_value) (break `/Game/InventorySystem/Structures/Struct_Item` (`self.ItemStructure`)))
  (`parent.Use`)
  (bind _asthird_person_character_1 (cast `/Game/Astra/ThirdPersonCharacter1` (`GameplayStatics.GetPlayerCharacter` 0)))
  (set `/Game/Astra/ThirdPersonCharacter1.CurrentHealth` (+ (`/Game/Astra/ThirdPersonCharacter1.CurrentHealth` _asthird_person_character_1) _itemstructure_value) _asthird_person_character_1)
  (return true))

(fn `UserConstructionScript`
  (`parent.UserConstructionScript`))