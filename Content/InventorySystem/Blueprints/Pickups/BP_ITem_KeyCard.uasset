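; Key card item pickup in the inventory system that adds a key to the player.
; When the actor ends play, it casts player character 0 to Astra and increments KeyCount.
; The count relies on EndPlay as the collection signal and does not check the end reason, so any removal of the actor triggers it.
; The Use function is empty.
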(event `self.ReceiveEndPlay`
  (params (EndPlayReason :type "EEndPlayReason Enum" :default "Destroyed"))
  ;[1 1 1] When the key card is collected and destroyed, increased the number of keys the player has.
  ; (DAN work, implemented into this BP)
  (bind _asastra (cast `/Game/Astra/Astra` (`GameplayStatics.GetPlayerCharacter` 0)))
  (set `/Game/Astra/Astra.KeyCount` (+ (`/Game/Astra/Astra.KeyCount` _asastra) 1) _asastra))

(fn `Use`)

(fn `UserConstructionScript`
  (`parent.UserConstructionScript`))