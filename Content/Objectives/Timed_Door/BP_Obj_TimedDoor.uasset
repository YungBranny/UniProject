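; Timed door objective: a locked door that unlocks when the player turns on enough BP_Switch actors before a countdown expires.
; Once IsObjectiveTriggered is set, Tick shows the timer widget, counts down through a Delay and checks Astra's switch count.
; Failure resets the switches and timer for a retry; success plays a sound and popup and unlocks the door.
; Overlap boxes drive the Timeline door slide and the player-facing locked-door prompt.
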(event `self.ReceiveBeginPlay`
  (set `self.bCanBeDamaged` false)
  ;[1 0 1] Set isDoorLocked to True
  (set `self.isDoorLocked` true)
  ;[1 0 1] Set the InteractionText to not visible
  (`SceneComponent.SetVisibility` (`self.InteractionText`) false false)
  ;[1 1 1] Create widget of objective timer and set visibility to hidden
  (bind _returnvalue (`|CreateWidget` "/Game/Objectives/Timed_Door/W_ObjTimer.W_ObjTimer_C"))
  (bind _output_get (set `self.W_ObjTimer` _returnvalue))
  (`UserWidget.AddToViewport` _output_get 0)
  (`Widget.SetVisibility` _output_get "Hidden")
  ;[1 1 1] Cast to Astra and promote to variable
  (bind _asastra (cast `/Game/Astra/Astra` (`GameplayStatics.GetPlayerCharacter` 0)))
  (set `self.Astra` _asastra)
  ;[1 1 1] Set the seconds (used for timer)
  (set `self.Seconds` (`self.Timer_Seconds`)))

(event `self.ReceiveTick`
  (params (DeltaSeconds :type "Float (single-precision)"))
  (bind _interactiontext (`self.InteractionText`))
  (bind _w_popuptext (`/Game/Astra/Astra.W_PopUpText` (`self.Astra`)))
  (bind _w_popuptext_2 (`/Game/Astra/Astra.W_PopUpText` (`self.Astra`)))
  ;[1 0 1] Set the rotation of theInteractionText to facing the player
  (`SceneComponent.K2_SetWorldRotation` _interactiontext (`KismetMathLibrary.FindLookAtRotation` (`SceneComponent.K2_GetComponentLocation` _interactiontext) (`self.K2_GetActorLocation` (`GameplayStatics.GetPlayerPawn` 0))) false false)
  (`|ExecutionSequence`
    (:`then_0`
      ;[1 1 1] If the objective has been triggered
      (if (`self.isObjectiveTriggered`)
        ;[1 1 1] Set the payers objective
        (set `/Game/Astra/Astra.PlayerObjectives` (`KismetTextLibrary.Conv_StringToText` (`self.PlayerObjectiveText`)) (`self.Astra`))
        ;[1 1 1] Show the timer
        (`Widget.SetVisibility` (`self.W_ObjTimer`) "Visible")
        ;[1 1 1] Start the timer for the objective
        (`KismetSystemLibrary.Delay` 1.0)
        (bind _istimerfinished (`self.Timer`))))
    (:`then_1`
      ;[1 1 1] If the timer has finished
      (if _istimerfinished
        ;[1 1 1] If the number of switches that the player has turned on (SwitchUnlockedCount) is not equal to the number required for the objective
        (if (!= (`/Game/Astra/Astra.SwitchUnlockedCount` (`self.Astra`)) (`self.SwitchesUnlockedRequired`))
          ;[1 1 1] Set the objective triggered to false
          (set `self.isObjectiveTriggered` false)
          ;[1 1 1] Go through all the switches and turn them off
          (bind _outactors (`GameplayStatics.GetAllActorsOfClass` "/Game/Objectives/Timed_Door/BP_Switch.BP_Switch_C"))
          (for _array_element _outactors
            (if (`/Game/Objectives/Timed_Door/BP_Switch.isSwitchedOn` _array_element)
              (`/Game/Objectives/Timed_Door/BP_Switch.SwitchOff` _array_element)))
          ;[1 1 1] Reset the values, ready for doing the objective again
          (set `/Game/Astra/Astra.SwitchUnlockedCount` 0 (`self.Astra`))
          (set `/Game/Astra/Astra.PlayerObjectives` (`KismetTextLibrary.Conv_StringToText` (`self.ObjectiveFailedText`)) (`self.Astra`))
          (`Widget.SetVisibility` (`self.W_ObjTimer`) "Hidden")
          (set `self.Seconds` (+ (`self.Timer_Seconds`) 1)))))
    (:`then_2`
      ;[1 1 1] If the number of switches that the player has turned on (SwitchUnlockedCount) is equal to the number required for the objective
      (if (== (`/Game/Astra/Astra.SwitchUnlockedCount` (`self.Astra`)) (`self.SwitchesUnlockedRequired`))
        ;[1 1 1] Set isObjectiveComplete to true
        (set `self.isObjectiveComplete` true)))
    (:`then_3`
      ;[1 1 1] If isObjectiveComplete is true
      (if (`self.isObjectiveComplete`)
        (`|ExecutionSequence`
          (:`then_0`
            ;[1 1 1] Play sound to notify the player that the door has been unlocked
            (`/Engine/EditorBlueprintResources/StandardMacros.DoOnce` false
              (:`Completed`
                (`GameplayStatics.PlaySoundAtLocation` "/Game/Sound/Spacedoor_Open_Cue.Spacedoor_Open_Cue" (`SceneComponent.K2_GetComponentLocation` (`self.Door`)) (struct) 1.0 1.0 0.0 null null null)
                (`Widget.SetVisibility` _w_popuptext_2 "Visible")
                (`TextBlock.SetText` (`/Game/GUI/W_PopUpText.T_PopUpText` _w_popuptext_2) "The door has unlocked!")
                (`KismetSystemLibrary.Delay` 3.0)
                (`TextBlock.SetText` (`/Game/GUI/W_PopUpText.T_PopUpText` _w_popuptext) "")
                (`Widget.SetVisibility` _w_popuptext "Hidden"))))
          (:`then_1`
            (`Widget.SetVisibility` (`self.W_ObjTimer`) "Hidden")
            (set `self.Seconds` (+ (`self.Timer_Seconds`) 1))
            (set `/Game/Astra/Astra.PlayerObjectives` "" (`self.Astra`)))
          (:`then_2`
            ;;[1 1 1] Set isDoorLocked to false
            (set `self.isDoorLocked` false)))))))

(event `self.Box.OnComponentBeginOverlap`
  (params (OverlappedComponent :type "PrimitiveComponent Object Reference") (OtherActor :type "Actor Object Reference") (OtherComp :type "PrimitiveComponent Object Reference") (OtherBodyIndex :type Integer) (bFromSweep :type Boolean) (SweepResult :type "HitResult Structure (by ref)"))
  ;[1 1 1] Door opens and closes when player enters and exits box trigger
  (cast `/Game/Astra/Astra` OtherActor)
  (if (not (`self.isDoorLocked`))
    (bind (_direction _movedoor) (`Timeline|Timeline_0` :!label _label)
      (:`Update`
        (`SceneComponent.K2_SetRelativeLocation` (`self.Door`) (`KismetMathLibrary.VLerp` (0.0 0.0 0.0) (`self.TargetLocation`) _movedoor) false false)))))

(event `self.Box.OnComponentEndOverlap`
  (params (OverlappedComponent :type "PrimitiveComponent Object Reference") (OtherActor :type "Actor Object Reference") (OtherComp :type "PrimitiveComponent Object Reference") (OtherBodyIndex :type Integer))
  ;[1 1 1] Door opens and closes when player enters and exits box trigger
  (cast `/Game/Astra/Astra` OtherActor)
  (goto _label :!via `Reverse`))

(event `self.InteractText.OnComponentBeginOverlap`
  (params (OverlappedComponent :type "PrimitiveComponent Object Reference") (OtherActor :type "Actor Object Reference") (OtherComp :type "PrimitiveComponent Object Reference") (OtherBodyIndex :type Integer) (bFromSweep :type Boolean) (SweepResult :type "HitResult Structure (by ref)"))
  (bind _interactiontext (`self.InteractionText`))
  ;[1 0 1] If the player is in the InteractText box collision, check to see if the InteractionText should be visible or not.
  (cast `/Game/Astra/Astra` OtherActor)
  (if (== (`self.isDoorLocked`) true)
    (`SceneComponent.SetVisibility` _interactiontext true false) ; Set the InteractionText to not be visible
    (else
      (`SceneComponent.SetVisibility` _interactiontext false false) ; Set the InteractionText to be visible
    )))

(event `self.InteractText.OnComponentEndOverlap`
  (params (OverlappedComponent :type "PrimitiveComponent Object Reference") (OtherActor :type "Actor Object Reference") (OtherComp :type "PrimitiveComponent Object Reference") (OtherBodyIndex :type Integer))
  ;[1 0 1] If the player is not in the InteractText box collision, set the InteractionText to not be visible
  (cast `/Game/Astra/Astra` OtherActor)
  (`SceneComponent.SetVisibility` (`self.InteractionText`) false false)
  (`Widget.SetVisibility` (`/Game/Astra/Astra.W_PopUpText` (`self.Astra`)) "Hidden"))

(fn `Timer`
  (returns (isTimerFinished :type Boolean))
  ;[1 1 1] Decrease seconds by 1
  (set `self.Seconds` (- (`self.Seconds`) 1))
  ;[1 1 1] Return if seconds is less than or equal to 0
  (return (<= (`self.Seconds`) 0)))

(fn `UserConstructionScript`)