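; BP_Switch is a switch actor for the timed door objective that starts locked and cannot be damaged.
; Every Tick it hides its static mesh while IsLocked is false; nothing in this graph clears that flag.
; ActivateOutline and DeactivateOutline events toggle a custom depth stencil on the mesh for an outline highlight.
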(event `self.ReceiveBeginPlay`
  (set `self.bCanBeDamaged` false)
  (set `self.isLocked` true))

(event `self.ReceiveTick`
  (params (DeltaSeconds :type "Float (single-precision)"))
  (if (not (`self.isLocked`))
    (`SceneComponent.SetVisibility` (`self.StaticMesh`) false false)))

(event `/Game/Interfaces/Interface_Object_Outline.ActivateOutline`
  (bind _staticmesh (`self.StaticMesh`))
  (`PrimitiveComponent.SetRenderCustomDepth` _staticmesh true)
  (`PrimitiveComponent.SetCustomDepthStencilValue` _staticmesh 1))

(event `/Game/Interfaces/Interface_Object_Outline.DeactivateOutline`
  (`PrimitiveComponent.SetRenderCustomDepth` (`self.StaticMesh`) false))

(fn `UserConstructionScript`)