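; BP_TimedDoor is a sliding door that opens for Astra only while unlocked.
; It starts locked, and nothing here unlocks it or runs a timer.
; Box overlap plays a timeline that lerps the door toward TargetLocation, and leaving reverses it.
; InteractionText starts hidden and faces the player each tick, but its key-count visibility check is disconnected, so this graph never shows it.
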(event `self.ReceiveBeginPlay`
  (set `self.bCanBeDamaged` false)
  ;[1 0 1] Set isDoorLocked to True
  (set `self.isDoorLocked` true)
  ;[1 0 1] Set the InteractionText to not visible
  (`SceneComponent.SetVisibility` (`self.InteractionText`) false false))

(event `self.ReceiveTick`
  (params (DeltaSeconds :type "Float (single-precision)"))
  (bind _interactiontext (`self.InteractionText`))
  ;[1 0 1] Set the rotation of theInteractionText to facing the player
  (`SceneComponent.K2_SetWorldRotation` _interactiontext (`KismetMathLibrary.FindLookAtRotation` (`SceneComponent.K2_GetComponentLocation` _interactiontext) (`self.K2_GetActorLocation` (`GameplayStatics.GetPlayerPawn` 0))) false false))

(event `self.Box.OnComponentBeginOverlap`
  (params (OverlappedComponent :type "PrimitiveComponent Object Reference") (OtherActor :type "Actor Object Reference") (OtherComp :type "PrimitiveComponent Object Reference") (OtherBodyIndex :type Integer) (bFromSweep :type Boolean) (SweepResult :type "HitResult Structure (by ref)"))
  ;[1 1 1] Door opens and closes when player enters and exits box trigger
  (cast `/Game/Astra/Astra` OtherActor)
  (if (not (`self.isDoorLocked`))
    (bind (_direction _movedoor) (`Timeline|Timeline_0` :!label _label)
      (:`Update`
        (`SceneComponent.K2_SetRelativeLocation` (`self.Door`) (`KismetMathLibrary.VLerp` (0.0 0.0 0.0) (`self.TargetLocation`) _movedoor) false false)))))

(event `self.Box.OnComponentEndOverlap`
  (params (OverlappedComponent :type "PrimitiveComponent Object Reference") (OtherActor :type "Actor Object Reference") (OtherComp :type "PrimitiveComponent Object Reference") (OtherBodyIndex :type Integer))
  ;[1 1 1] Door opens and closes when player enters and exits box trigger
  (cast `/Game/Astra/Astra` OtherActor)
  (goto _label :!via `Reverse`))

(event `self.InteractText.OnComponentBeginOverlap`
  (params (OverlappedComponent :type "PrimitiveComponent Object Reference") (OtherActor :type "Actor Object Reference") (OtherComp :type "PrimitiveComponent Object Reference") (OtherBodyIndex :type Integer) (bFromSweep :type Boolean) (SweepResult :type "HitResult Structure (by ref)"))
  ;[1 0 1] If the player is in the InteractText box collision, check to see if the InteractionText should be visible or not.
  (cast `/Game/Astra/Astra` OtherActor))

(event `self.InteractText.OnComponentEndOverlap`
  (params (OverlappedComponent :type "PrimitiveComponent Object Reference") (OtherActor :type "Actor Object Reference") (OtherComp :type "PrimitiveComponent Object Reference") (OtherBodyIndex :type Integer))
  ;[1 0 1] If the player is not in the InteractText box collision, set the InteractionText to not be visible
  (cast `/Game/Astra/Astra` OtherActor)
  (`SceneComponent.SetVisibility` (`self.InteractionText`) false false))

(fn `UserConstructionScript`)