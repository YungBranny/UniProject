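; Teleporter Blueprint that moves the player to a destination when the Astra character overlaps its box.
; After a one-second delay, it sets player character 0's location to the world position of the TeleportTo component, an arrow marking the end point.
; It then plays the Teleport_Mode_Entered sound at the world origin.
; An unused older version, originally from the Level Blueprint, remains in the graph.
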(event `self.Box.OnComponentBeginOverlap`
  (params (OverlappedComponent :type "PrimitiveComponent Object Reference") (OtherActor :type "Actor Object Reference") (OtherComp :type "PrimitiveComponent Object Reference") (OtherBodyIndex :type Integer) (bFromSweep :type Boolean) (SweepResult :type "HitResult Structure (by ref)"))
  (bind (_returnvalue_x _returnvalue_y _returnvalue_z) (`KismetMathLibrary.BreakVector` (`SceneComponent.K2_GetComponentLocation` (`self.TeleportTo`))))
  ;[1 1 1] Once Player overlaps Teleport box, there is a delay then it sets the new Player Location to where the arrow, which is the end point, has been moved.
  (cast `/Game/Astra/Astra` OtherActor)
  (`KismetSystemLibrary.Delay` 1.0)
  (`self.K2_SetActorLocation` (`GameplayStatics.GetPlayerCharacter` 0) (`KismetMathLibrary.MakeVector` _returnvalue_x _returnvalue_y _returnvalue_z) false false)
  (`GameplayStatics.PlaySoundAtLocation` "/Engine/VREditor/Sounds/UI/Teleport_Mode_Entered.Teleport_Mode_Entered" (0.0 0.0 0.0) (struct) 1.0 1.0 0.0 null null null))

(fn `UserConstructionScript`)