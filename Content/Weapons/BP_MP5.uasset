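; MP5 weapon for the Astra player character: automatic hitscan fire that spends Astra's battery as ammo.
; Fire traces from the ADS camera with random recoil spread, reports the shot, then applies damage with blood or leaves metal impacts and bullet-hole decals.
; A timeline kicks the view, and Fire re-calls itself through a retriggerable delay while shooting.
; Blood particle collisions spawn randomized splatter decals through dynamic material instances.
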(event `self.ReceiveBeginPlay`
  ;[1 1 1] Cast to astra
  (bind _asastra (cast `/Game/Astra/Astra` (`GameplayStatics.GetPlayerCharacter` 0)))
  (set `self.Astra` _asastra))

(event `/Game/GunInterface.Fire`
  (bind _returnvalue (`GameplayStatics.GetPlayerCharacter` 0))
  (bind _astra (`self.Astra`))
  (bind _returnvalue_2 (`SceneComponent.K2_GetComponentLocation` (`self.Shoot Point`)))
  (bind _adscamera (`/Game/Astra/Astra.ADSCamera` (`self.Astra`)))
  (bind _recoilsmg (`/Game/Astra/Astra.RecoilSMG` (`self.Astra`)))
  (bind _returnvalue_3 (`SceneComponent.K2_GetComponentLocation` _adscamera))
  (bind _returnvalue_4 (* _recoilsmg -1.0))
  ;[1 1 1] MP5 shoot function
  (set `/Game/Astra/Astra.Decrease Battery Amount` 1.0 _astra)
  (if (<= (`/Game/Astra/Astra.CurrentBattery` _astra) 0.0)
    (`GameplayStatics.PlaySoundAtLocation` "/Game/Sound/lowammo_01.lowammo_01" (`self.K2_GetActorLocation`) (struct) 1.0 1.0 0.0 null null null)
    (else
      (`/Game/Astra/Astra.Battery Decrease Bullet` (`self.Astra`))
      (`GameplayStatics.SpawnEmitterAtLocation` "/Game/SciFiWeapLight/FX/Particles/P_Pistol_MuzzleFlash_Dark.P_Pistol_MuzzleFlash_Dark" _returnvalue_2 (`self.K2_GetActorRotation`))
      (`GameplayStatics.PlaySoundAtLocation` "/Game/SciFiWeapLight/Sound/Pistol/Pistol_Fire_Cue.Pistol_Fire_Cue" _returnvalue_2 (struct) 1.0 1.0 0.0 null null null)
      (`GameplayStatics.PlayWorldCameraShake` "/Game/SMG_Shake.SMG_Shake_C" _returnvalue_3 0.0 500.0)
      (bind (_outhit _returnvalue_5) (`KismetSystemLibrary.LineTraceSingle` _returnvalue_3 (+ (+ _returnvalue_3 (* (`SceneComponent.GetForwardVector` _adscamera) 60000.0)) (`KismetMathLibrary.MakeVector` (`KismetMathLibrary.RandomFloatInRange` _returnvalue_4 _recoilsmg) (`KismetMathLibrary.RandomFloatInRange` _returnvalue_4 _recoilsmg) (`KismetMathLibrary.RandomFloatInRange` _returnvalue_4 _recoilsmg))) "TraceTypeQuery1"))
      (`|ExecutionSequence`
        (:`then_0`
          (if _returnvalue_5
            (bind (_bblockinghit _binitialoverlap _time _distance _location _impactpoint _normal _impactnormal _physmat _hitactor _hitcomponent _hitbonename _hititem _faceindex _tracestart) (`GameplayStatics.BreakHitResult` _outhit))
            (message `/Game/Ai/BossNPC/CollisionDetection.OnHit` _hitactor _impactpoint)
            (`/Engine/EditorBlueprintResources/StandardMacros.IsValid` _hitactor
              (:`Is Valid`
                _)
              (:`Is Not Valid`
                _))
            (`AISense_Damage.ReportDamageEvent` _hitactor (`GameplayStatics.GetPlayerCharacter` 0) 1.0 _tracestart)
            (if (`Actor.bCanBeDamaged` _hitactor)
              (bind _returnvalue_6 (`KismetMathLibrary.MakeRotFromX` _normal))
              (`GameplayStatics.SpawnEmitterAtLocation` "/Game/StarterContent/Particles/Blood.Blood" _impactpoint _returnvalue_6 (3.0 3.0 3.0))
              (bind _returnvalue_7 (`GameplayStatics.SpawnEmitterAtLocation` "/Game/P_Splatter.P_Splatter" _impactpoint _returnvalue_6 (3.0 3.0 3.0)))
              (add `ParticleSystemComponent.OnParticleCollide` _returnvalue_7 (delegate `OnCollideBlood`))
              (`GameplayStatics.ApplyDamage` _hitactor 7.0 null (`GameplayStatics.GetPlayerCharacter` 0))
              (else
                (`GameplayStatics.SpawnEmitterAtLocation` "/Game/SciFiWeapLight/FX/Particles/P_Impact_Metal_Medium_Dark.P_Impact_Metal_Medium_Dark" _impactpoint _returnvalue_6)
                (bind _returnvalue_8 (`GameplayStatics.SpawnDecalAtLocation` "/Game/Decal_Bullet_Hole.Decal_Bullet_Hole" (10.0 10.0 10.0) _impactpoint _returnvalue_6 10.0))
                (`DecalComponent.SetFadeScreenSize` _returnvalue_8 0.0)
                (`SceneComponent.K2_AttachToComponent` _returnvalue_8 _hitcomponent "None" "KeepWorld" "KeepWorld" "KeepWorld" true)
                (`GameplayStatics.PlaySoundAtLocation` "/Game/Sound/Rico.Rico" _impactpoint (struct) 1.0 1.0 0.0 null null null)))))
        (:`then_1`
          (`Timeline|Timeline_0`
            (:`Update`
              (`Pawn.AddControllerYawInput` _returnvalue (`KismetMathLibrary.RandomFloatInRange` -0.15 0.15))
              (`Pawn.AddControllerPitchInput` _returnvalue (`KismetMathLibrary.RandomFloatInRange` -0.5 -0.5)))))
        (:`then_2`
          ;[1 1 1] Looping the fire-rate
          (if (`/Game/Astra/Astra.isShootingMP5` (`self.Astra`))
            (`KismetSystemLibrary.RetriggerableDelay` (`/Game/Astra/Astra.FireRate` (`self.Astra`)))
            (`/Game/GunInterface.Fire`)))))))

(event `OnCollideBlood`
  (params (EventName :type Name) (EmitterTime :type "Float (double-precision)") (ParticleTime :type Integer) (Location :type "Vector Structure") (Velocity :type "Vector Structure") (Direction :type "Vector Structure") (Normal :type "Vector Structure") (BoneName :type Name) (PhysMat :type "PhysicalMaterial Object Reference"))
  ;[1 1 1] MP5 shoot function
  (bind _returnvalue (`KismetMaterialLibrary.CreateDynamicMaterialInstance` "/Game/Splatter_Decal.Splatter_Decal"))
  (`MaterialInstanceDynamic.SetScalarParameterValue` _returnvalue "Frame" (`KismetMathLibrary.Conv_IntToDouble` (`KismetMathLibrary.RandomInteger` 11)))
  (`GameplayStatics.SpawnDecalAtLocation` _returnvalue (`KismetMathLibrary.Conv_DoubleToVector` (`KismetMathLibrary.RandomFloatInRange` 10.0 30.0)) Location (`KismetMathLibrary.Conv_VectorToRotator` Normal) 15.0))

(fn `UserConstructionScript`)